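; Magic link VFX actor that draws a Niagara beam from itself to an end actor, a fixed location, or its own SelfEnd point in self-end mode.
; Construction script pushes width, color, tangent and timing into the start, link and end effects.
; Tick updates the end position, applies toggle changes, optionally scales tiling by distance, and spins the arrow in self-end mode.
; An optional interval-throttled line trace spawns hit effects.
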(event EventBeginPlay
  (bind _linkvfx (Variables|Default|GetLinkVFX))
  (bind _endactor (Variables|Default|GetEndActor))
  (bind _endvfx (Variables|Default|GetEndVFX))
  (Utilities|FlowControl|Sequence
    (:then_0
      ;[1 1 1] Initial
      (if (Variables|Default|GetSelfEndMode)
        (Variables|Default|SetMyEndPos (Transformation|GetWorldLocation (Variables|Default|GetSelfEnd)))
        (elif (Utilities|IsValid _endactor)
          (Variables|Default|SetMyEndPos (Transformation|GetWorldLocation (Variables|/Script/Engine.Actor|GetRootComponent _endactor)))
          (else
            (Variables|Default|SetMyEndPos (Variables|Default|GetEndLocation)))))
      (Components|Activation|SetActive (Variables|Default|GetStartVFX) (and (Variables|Default|GetLinkVfxOn) (Variables|Default|GetStartVfxOn)) true)
      (Variables|Default|SetStartVfxOn_State (Variables|Default|GetStartVfxOn)))
    (:then_1
      (Components|Activation|SetActive _linkvfx (Variables|Default|GetLinkVfxOn) true)
      (Variables|Default|SetLinkVfxOn_State (Variables|Default|GetLinkVfxOn))
      (Niagara|SetNiagaraVariable(Vector3) _linkvfx "EndPos_V" (Variables|Default|GetMyEndPos)))
    (:then_2
      (Components|Activation|SetActive _endvfx (and (Variables|Default|GetLinkVfxOn) (Variables|Default|GetEndVfxOn)) true)
      (Variables|Default|SetEndVfx_State (Variables|Default|GetEndVfxOn))
      (Transformation|SetWorldLocation _endvfx (Variables|Default|GetMyEndPos) false false))))

(event EventTick
  (params (DeltaSeconds :type Float%20%28single-precision%29))
  (bind _linkvfx (Variables|Default|GetLinkVFX))
  (bind _endvfx (Variables|Default|GetEndVFX))
  (bind _linkvfx_2 (Variables|Default|GetLinkVFX))
  (bind _startvfx (Variables|Default|GetStartVFX))
  (bind _endactor (Variables|Default|GetEndActor))
  (Utilities|FlowControl|Sequence
    (:then_0
      ;[1 1 1] EndPosControl
      (if (Variables|Default|GetSelfEndMode)
        (Variables|Default|SetMyEndPos (Transformation|GetWorldLocation (Variables|Default|GetSelfEnd)))
        (elif (Utilities|IsValid _endactor)
          (Variables|Default|SetMyEndPos (Transformation|GetWorldLocation (Variables|/Script/Engine.Actor|GetRootComponent _endactor)))
          (else
            (Variables|Default|SetMyEndPos (Variables|Default|GetEndLocation)))))
      ;[1 1 1] StartVfxControl
      (if (or (!= (Variables|Default|GetStartVfxOn) (Variables|Default|GetStartVfxOn_State)) (!= (Variables|Default|GetLinkVfxOn) (Variables|Default|GetLinkVfxOn_State)))
        (if (and (Variables|Default|GetLinkVfxOn) (Variables|Default|GetStartVfxOn))
          (Components|Activation|SetActive _startvfx true true)
          (else
            (Components|Activation|SetActive _startvfx false true)))
        (Variables|Default|SetStartVfxOn_State (Variables|Default|GetStartVfxOn))))
    (:then_1
      ;[1 1 1] EndVfxControl
      (if (Variables|Default|GetEndVfxOn)
        (Transformation|SetWorldLocation _endvfx (Variables|Default|GetMyEndPos) false false))
      (if (or (!= (Variables|Default|GetEndVfxOn) (Variables|Default|GetEndVfx_State)) (!= (Variables|Default|GetLinkVfxOn) (Variables|Default|GetLinkVfxOn_State)))
        (if (and (Variables|Default|GetLinkVfxOn) (Variables|Default|GetEndVfxOn))
          (Components|Activation|SetActive _endvfx true true)
          (else
            (Components|Activation|SetActive _endvfx false true)))
        (Variables|Default|SetEndVfx_State (Variables|Default|GetEndVfxOn))))
    (:then_2
      ;[1 1 1] LinkVfxControl
      (Niagara|SetNiagaraVariable(Vector3) _linkvfx "EndPos_V" (Variables|Default|GetMyEndPos))
      (if (Variables|Default|GetU_Tile_AutoScale)
        (Niagara|SetNiagaraVariable(Float) _linkvfx "U_Tile_Scale" (/ (Math|Vector|Distance(Vector) (Variables|Default|GetMyEndPos) (Transformation|GetActorLocation)) (Variables|Default|GetU_Tile_AutoScaleControl))))
      (if (!= (Variables|Default|GetLinkVfxOn) (Variables|Default|GetLinkVfxOn_State))
        (if (Variables|Default|GetLinkVfxOn)
          (if (Components|Activation|IsActive _linkvfx_2)
            _
            (else
              _))
          (Components|Activation|SetActive _linkvfx_2 true true)
          (else
            (Components|Activation|SetActive _linkvfx_2 false true)))
        (Variables|Default|SetLinkVfxOn_State (Variables|Default|GetLinkVfxOn))))
    (:then_3
      ;[1 1 1] SelfRotate
      (if (Variables|Default|GetSelfEndMode)
        (Transformation|AddRelativeRotation (Variables|Default|GetArrow) (Math|Rotator|MakeRotator 0.0 0.0 (Variables|Default|GetSelfRoationSpeed)) false false)))
    (:then_4
      ;[1 1 1] SelfHit
      (if (and (Variables|Default|GetCanHitState) (Variables|Default|GetCanHit))
        (bind (_outhit _returnvalue) (Collision|LineTraceForObjects (Transformation|GetActorLocation) (Variables|Default|GetMyEndPos) (Variables|Default|GetSelfTargetTypes) false 0 "None"))
        (Variables|Default|SetCanHitState (not _returnvalue))
        (Niagara|SpawnSystematLocation (Variables|Default|GetHitVFX) (.ImpactPoint (Collision|BreakHitResult _outhit)) "0, 0, 0" "1.000000,1.000000,1.000000" true _returnvalue)
        (Utilities|FlowControl|Delay (Variables|Default|GetHit_Interval))
        (Variables|Default|SetCanHitState true)))))

(fn ConstructionScript
  (bind _selfradius (Variables|Default|GetSelfRadius))
  (bind _linkvfx (Variables|Default|GetLinkVFX))
  (bind _endvfx (Variables|Default|GetEndVFX))
  (bind _startvfx (Variables|Default|GetStartVFX))
  (bind _endactor (Variables|Default|GetEndActor))
  (bind _box2 (Variables|Default|GetBox2))
  (bind _returnvalue (* _selfradius 0.5))
  (Utilities|FlowControl|Sequence
    (:then_0
      ;[1 1 1] Base_Initial
      (Rendering|SetVisibility (Variables|Default|GetBox2) (Variables|Default|GetSelfEndMode) false)
      (Transformation|SetRelativeLocation (Variables|Default|GetSelfEnd) (Math|Vector|MakeVector (Variables|Default|GetSelfRadius) 0.0 0.0) false false)
      (Transformation|SetRelativeLocation _box2 (Math|Vector|MakeVector _returnvalue 0.0 0.0) false false)
      (Components|Box|SetBoxExtent _box2 (Math|Vector|MakeVector _returnvalue 35.0 35.0) true)
      (if (Variables|Default|GetSelfEndMode)
        (Variables|Default|SetMyEndPos (Transformation|GetWorldLocation (Variables|Default|GetSelfEnd)))
        (elif (Utilities|IsValid _endactor)
          (Variables|Default|SetMyEndPos (Transformation|GetWorldLocation (Variables|/Script/Engine.Actor|GetRootComponent _endactor)))
          (else
            (Variables|Default|SetMyEndPos (Variables|Default|GetEndLocation))))))
    (:then_1
      ;[1 1 1] LinkVfx_Initial
      (Components|Activation|SetAutoActivate _linkvfx (Variables|Default|GetLinkVfxOn))
      (Niagara|SetNiagaraVariable(Vector3) _linkvfx "EndPos_V" (Variables|Default|GetMyEndPos))
      (Niagara|SetNiagaraVariable(Float) _linkvfx "_Width" (Variables|Default|GetWidth))
      (Class|NiagaraComponent|SetVariableBool _linkvfx "DontConnect" (Variables|Default|GetSelfEndMode))
      (Niagara|SetNiagaraVariable(Float) _linkvfx "EndTangent" (Variables|Default|GetTangentEnd))
      (Niagara|SetNiagaraVariable(Float) _linkvfx "TransitionTime" (Variables|Default|GetTransitionTime))
      (Class|NiagaraComponent|SetVariableBool _linkvfx "AudioOn" (Variables|Default|GetAudioOn))
      (Class|NiagaraComponent|SetVariableBool _linkvfx "HeadVFX" (Variables|Default|GetHeadVfxOn%28Static%29))
      (Niagara|SetNiagaraVariable(Float) _linkvfx "_ColorHue" (Variables|Default|GetColorHue)))
    (:then_2
      ;[1 1 1] EndVfx_Initial
      (Components|Activation|SetAutoActivate _endvfx (and (Variables|Default|GetEndVfxOn) (Variables|Default|GetLinkVfxOn)))
      (Transformation|SetWorldLocation _endvfx (Variables|Default|GetMyEndPos) false false)
      (Niagara|SetNiagaraVariable(Float) _endvfx "CameraOffset" (Variables|Default|GetTipVfxCameraOffset))
      (Niagara|SetNiagaraVariable(Float) _endvfx "_ColorHue" (Variables|Default|GetColorHue))
      (Niagara|SetNiagaraVariable(Float) _endvfx "_Width" (Variables|Default|GetWidth))
      (Niagara|SetNiagaraVariable(Float) (Variables|Default|GetEndVFX) "DelayTime" (Variables|Default|GetTransitionTime)))
    (:then_3
      ;[1 1 1] StartVfx_Initial
      (Components|Activation|SetAutoActivate _startvfx (and (Variables|Default|GetStartVfxOn) (Variables|Default|GetLinkVfxOn)))
      (Niagara|SetNiagaraVariable(Float) _startvfx "CameraOffset" (Variables|Default|GetTipVfxCameraOffset))
      (Niagara|SetNiagaraVariable(Float) _startvfx "_ColorHue" (Variables|Default|GetColorHue)))))