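; BP_Building8 is a modular building prop for the stylized city, with optional variations on its left and right sides.
; The construction script reads the Left and Right flags and, for each enabled side, hides two wall meshes and shows two block meshes in their place.
; The event graph holds only disabled placeholder events, so the building has no runtime logic.
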(event EventBeginPlay)

(event Collision|EventActorBeginOverlap
  (params (OtherActor :type Actor%20Object%20Reference)))

(event EventTick
  (params (DeltaSeconds :type Float%20%28single-precision%29)))

(fn ConstructionScript
  (if (Variables|Default|GetLeft)
    (Rendering|SetVisibility (Variables|Default|GetSM_Wall24_StaticMeshComponent0) false false)
    (Rendering|SetVisibility (Variables|Default|GetSM_BlockC27_StaticMeshComponent1) true false))
  (if (Variables|Default|GetRight)
    (Rendering|SetVisibility (Variables|Default|GetSM_Wall14_StaticMeshComponent0) false false)
    (Rendering|SetVisibility (Variables|Default|GetSM_BlockC73_StaticMeshComponent1) true false)))