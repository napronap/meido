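; BP_Building10 is a stylized city building assembled from static mesh components, with configurable left and right sides.
; In the Construction Script, the Left and Right booleans each hide that side's wall meshes and show a matching set of block meshes.
; Each flag only applies the swap when true, and the event graph has no runtime logic.
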(event EventBeginPlay)

(event Collision|EventActorBeginOverlap
  (params (OtherActor :type Actor%20Object%20Reference)))

(event EventTick
  (params (DeltaSeconds :type Float%20%28single-precision%29)))

(fn ConstructionScript
  (if (Variables|Default|GetLeft)
    (Rendering|SetVisibility (Variables|Default|GetSM_Wall124_StaticMeshComponent0) false false)
    (Rendering|SetVisibility (Variables|Default|GetSM_BlockC2B7_StaticMeshComponent3) true false))
  (if (Variables|Default|GetRight)
    (Rendering|SetVisibility (Variables|Default|GetSM_Wall92_StaticMeshComponent0) false false)
    (Rendering|SetVisibility (Variables|Default|GetSM_BlockC2B10_StaticMeshComponent5) true false)))