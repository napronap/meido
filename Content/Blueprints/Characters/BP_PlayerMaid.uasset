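; Player maid character Blueprint that drives the HUD, lock-on marker and menu presentation.
; BeginPlay creates both widgets, binds health, lock-on and controller flow-state events, and applies a menu pose montage with smiling face morphs.
; Entering Playing clears those morphs, plus others left by the C++ win-sequence camera transition, and shows the HUD, which Lose removes.
; Tick projects the locked target's location to screen space to position the marker.
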(event Custom|UpdateLockOnHUDVisibility
  (params (NewTarget :type Actor%20Object%20Reference) (bSuccess :type Boolean))
  (bind _lockonref (Variables|Default|GetLockOnRef))
  (if bSuccess
    (UserInterface|Viewport|AddtoViewport _lockonref 0)
    (else
      (Widget|RemovefromParent _lockonref))))

(event Custom|OnFlowStateChanged
  (params (NewState :type EFlowState%20Enum :default "MainMenu"))
  (bind _mesh (Variables|Character|GetMesh))
  (switch Utilities|FlowControl|Switch|SwitchonEFlowState NewState
    (:Playing
      ;[0.15 0.15 0.15 0.5] Cleanup from APlayerMaidCharacter::StartWinSequenceCameraTransition
      (Components|SkeletalMesh|SetMorphTarget _mesh "Fcl_EYE_Joy_R" 0.0 true)
      (Components|SkeletalMesh|SetMorphTarget _mesh "Fcl_MTH_Fun" 0.0 true)
      (Components|SkeletalMesh|SetMorphTarget _mesh "Fcl_MTH_Joy" 0.0 true)
      (Components|SkeletalMesh|SetMorphTarget _mesh "Fcl_EYE_Joy" 0.0 true)
      (UserInterface|Viewport|AddtoViewport (Variables|Default|GetHUDRef) 0))
    (:Lose
      (Widget|RemovefromParent (Variables|Default|GetHUDRef)))))

(event Custom|CustomEvent
  (params (HealthComponent :type Health%20Component%20Object%20Reference) (CurrentHealth :type Float%20%28single-precision%29) (MaxHealth :type Float%20%28single-precision%29) (Delta :type Float%20%28single-precision%29))
  (bind _hudref (Variables|Default|GetHUDRef))
  (Utilities|IsValid _hudref
    (:Is%20Valid
      (Variables|/Game/Blueprints/Widgets/WBP_PlayerHUD.WBP_PlayerHUD_C|SetCurrentHp _hudref CurrentHealth))))

(event EventBeginPlay
  (bind _mesh (Variables|Character|GetMesh))
  (bind _healthcomponent (Variables|Default|GetHealthComponent))
  (bind _maxhealth (Variables|/Script/meido_5_6.HealthComponent|GetMaxHealth _healthcomponent))
  (Utilities|FlowControl|Sequence
    (:then_0
      (bind _returnvalue (UserInterface|CreateWidget "/Game/Blueprints/Widgets/WBP_PlayerHUD.WBP_PlayerHUD_C"))
      (Variables|Default|SetHUDRef _returnvalue)
      (bind _returnvalue_2 (UserInterface|CreateWidget "/Game/Blueprints/Widgets/WBP_LockOnMarker.WBP_LockOnMarker_C"))
      (Variables|Default|SetLockOnRef _returnvalue_2))
    (:then_1
      (Variables|/Game/Blueprints/Widgets/WBP_PlayerHUD.WBP_PlayerHUD_C|SetMaxHp (Variables|Default|GetHUDRef) _maxhealth)
      (Variables|/Game/Blueprints/Widgets/WBP_PlayerHUD.WBP_PlayerHUD_C|SetCurrentHp (Variables|Default|GetHUDRef) _maxhealth))
    (:then_2
      (EventDispatchers|BindEventtoOnHealthChanged (Variables|Default|GetHealthComponent) (delegate Custom|CustomEvent)))
    (:then_3
      (EventDispatchers|BindEventtoOnLockonChanged (Variables|Default|GetLockOnComponent) (delegate Custom|UpdateLockOnHUDVisibility)))
    (:then_4
      (bind _asbp_maid_player_controller (Utilities|Casting|CastToBP_MaidPlayerController (Components|GetOwner)))
      (EventDispatchers|BindEventtoOnFlowStateChanged _asbp_maid_player_controller (delegate Custom|OnFlowStateChanged)))
    (:then_5
      (Animation|Montage|PlayMontage (Variables|Character|GetMesh) "/Game/Characters/Maid/Aki/Animations/Montages/AM_MainMenuPose.AM_MainMenuPose" 1.0 0.0 "PoseStart"))
    (:then_6
      (Components|SkeletalMesh|SetMorphTarget _mesh "Fcl_EYE_Joy_R" 1.0 true)
      (Components|SkeletalMesh|SetMorphTarget _mesh "Fcl_MTH_Fun" 0.6 true))))

(event EventTick
  (params (DeltaSeconds :type Float%20%28single-precision%29))
  (bind _lockoncomponent (Variables|Default|GetLockOnComponent))
  (bind _returnvalue (Class|LockonComponent|IsLockedon _lockoncomponent))
  (if _returnvalue
    (bind _returnvalue_2 (Class|LockonComponent|GetCurrentTarget _lockoncomponent))
    (bind _returnvalue_3 (Class|Targetable|GetTargetLocation(Message) _returnvalue_2))
    (Default|SetMarkerScreenPosition (Variables|Default|GetLockOnRef) (.ScreenPosition (Class|GameplayStatics|ProjectWorldtoScreen (Game|GetPlayerController 0) _returnvalue_3 true)))))

(fn ConstructionScript)